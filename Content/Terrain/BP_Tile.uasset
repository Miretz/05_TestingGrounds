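; BP_Tile is one segment of an infinite terrain that fills itself with random props (containers, boxes, canisters, rocks, sacks) on BeginPlay.
; Its barrier starts locked and red, and turns green and passable while the player is inside the locking volume.
; Leaving that volume relocks it and asks InfiniteTerrainGameMode to spawn a tile, while the delete volume destroys this one.
; GetAttachLocation exposes the Arrow's world transform as an attach point.
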(event `self.DeleteVolume.OnComponentBeginOverlap`
  (params (OverlappedComponent :type "PrimitiveComponent Object Reference") (OtherActor :type "Actor Object Reference") (OtherComp :type "PrimitiveComponent Object Reference") (OtherBodyIndex :type Integer) (bFromSweep :type Boolean) (SweepResult :type "HitResult Structure (by ref)"))
  ;[1 1 1] Delete
  (`self.IsPlayerActor` OtherActor)
  (`self.K2_DestroyActor`))

(event `self.ReceiveBeginPlay`
  ;[1 1 1] Lock on BeginPlay
  (`self.Lock`)
  (`self.PlaceActors` "/Game/Terrain/Props/BP_Container.BP_Container_C" 1 3)
  (`self.PlaceActors` "/Game/Terrain/Props/BP_Box.BP_Box_C" 2 4)
  (`self.PlaceActors` "/Game/Terrain/Props/BP_Canister.BP_Canister_C" 1 7)
  (`self.PlaceActors` "/Game/Terrain/Props/BP_Rock01.BP_Rock01_C" 0 4)
  (`self.PlaceActors` "/Game/Terrain/Props/BP_Rock05.BP_Rock05_C" 0 4)
  (`self.PlaceActors` "/Game/Terrain/Props/BP_Rock17.BP_Rock17_C" 0 4)
  (`self.PlaceActors` "/Game/Terrain/Props/BP_Sack.BP_Sack_C" 0 2))

(event `self.LockingVolume.OnComponentBeginOverlap`
  (params (OverlappedComponent :type "PrimitiveComponent Object Reference") (OtherActor :type "Actor Object Reference") (OtherComp :type "PrimitiveComponent Object Reference") (OtherBodyIndex :type Integer) (bFromSweep :type Boolean) (SweepResult :type "HitResult Structure (by ref)"))
  ;[1 1 1] Lock and Unlock
  (`self.IsPlayerActor` OtherActor)
  (`self.Unlock`))

(event `self.LockingVolume.OnComponentEndOverlap`
  (params (OverlappedComponent :type "PrimitiveComponent Object Reference") (OtherActor :type "Actor Object Reference") (OtherComp :type "PrimitiveComponent Object Reference") (OtherBodyIndex :type Integer))
  ;[1 1 1] Lock and Unlock
  (`self.IsPlayerActor` OtherActor)
  (`self.Lock`)
  (bind _asinfinite_terrain_game_mode (cast `/Game/InfiniteTerrainGameMode` (`GameplayStatics.GetGameMode`)))
  (`/Game/InfiniteTerrainGameMode.SpawnTile` _asinfinite_terrain_game_mode))

(fn `GetAttachLocation`
  (returns (AttachTransform :type "Transform Structure"))
  (return (`SceneComponent.K2_GetComponentToWorld` (`self.Arrow`))))

(fn `Lock`
  (`PrimitiveComponent.SetCollisionEnabled` (`self.Barrier`) "QueryAndPhysics")
  (`PrimitiveComponent.SetMaterial` (`self.Barrier`) 0 "/Game/Terrain/MI_Barrier_Red.MI_Barrier_Red"))

(fn `Unlock`
  (`PrimitiveComponent.SetCollisionEnabled` (`self.Barrier`) "NoCollision")
  (`PrimitiveComponent.SetMaterial` (`self.Barrier`) 0 "/Game/Terrain/MI_Barrier_Green.MI_Barrier_Green"))

(fn `UserConstructionScript`)